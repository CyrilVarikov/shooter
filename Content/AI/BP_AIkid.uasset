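; AI kid character that roams the level at random and heals the player on close contact.
; A self-repeating move event picks random navigable points around its current location, pausing briefly after each success or failure.
; When PawnSensing sees a TopDownCharacter inside the kid's actor bounds, it adds a small amount of clamped health and updates the health bar, with debug prints.
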(event `self.ReceiveBeginPlay`
  (`self.AidMoveToRndLoc`))

(event `AidMoveToRndLoc`
  ;[1 1 1] AI Random roam (aks teacher about on success and on fail)
  (`|AIMoveTo` self (`NavigationSystemV1.K2_GetRandomLocationInNavigableRadius` (`self.K2_GetActorLocation`) 500.0 null null) null
    (:`OnSuccess`
      _)
    (:`OnFail`
      _))
  (`KismetSystemLibrary.Delay` 1.0)
  (`self.AidMoveToRndLoc`))

(event `self.PawnSensing.OnSeePawn`
  (params (Pawn :type "Pawn Object Reference"))
  (bind (_origin _boxextent) (`self.GetActorBounds` false))
  (`KismetSystemLibrary.PrintString` "Hello")
  (bind _astop_down_character (cast `/Game/TopDownBP/Blueprints/TopDownCharacter` Pawn))
  (if (`KismetMathLibrary.IsPointInBox` (`self.K2_GetActorLocation` _astop_down_character) _origin _boxextent)
    (`KismetSystemLibrary.PrintString` "Hello")
    (bind _output_get (set `/Game/TopDownBP/Blueprints/TopDownCharacter.CurrentHealth` (`KismetMathLibrary.FClamp` (+ (`/Game/TopDownBP/Blueprints/TopDownCharacter.CurrentHealth` _astop_down_character) 5.0) 0.0 100.0) _astop_down_character))
    (`/Game/TopDownBP/Blueprints/TopDownCharacter.UpdateHealthBar` _astop_down_character _output_get)))

(fn `UserConstructionScript`)