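; AI controller for zombies that runs the BT_AI behavior tree and turns perception updates into blackboard state.
; Each sensed actor becomes AimActor if it is damageable and untagged as Zombie, unless the zombie is attacking or the player is in melee range.
; Stimuli are read by array index: the first sets CanSeePlayer, the second sets IsInvestigating and TargetLocation for hearing.
; Disconnected spawn, roam and perception-check nodes remain unused.
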(event `self.ReceiveBeginPlay`
  ;[1 1 1] Run tree
  (set `self.ControlledPawn` (`self.K2_GetPawn`))
  (`self.RunBehaviorTree` "/Game/AI/BT_AI.BT_AI"))

(event `self.ReceiveTick`
  (params (DeltaSeconds :type "Float (single-precision)"))
  ;[1 0.08854 0.08854] Probably this one is controlled by BT
)

(event `self.AIPerception.OnPerceptionUpdated`
  (params (UpdatedActors :type "Array of Actor Object Reference (by ref)"))
  (for _array_element UpdatedActors
    (bind _info (`AIPerceptionComponent.GetActorsPerception` (`self.AIPerception`) _array_element))
    (`self.CompleteSenses` (break `ActorPerceptionBlueprintInfo` _info) (`.LastSensedStimuli` (break `ActorPerceptionBlueprintInfo` _info)))))

(fn `CompleteSenses`
  (params (AimActor :type "Actor Object Reference") (Array :type "Array of AIStimulus Structure"))
  (`self.SetIfNotSelfAndNotSeeing` AimActor)
  (for (_array_element _array_index) Array
    (set `self.Stimulus` _array_element)
    (switch `int` _array_index
      (:`0`
        (`self.UpdateSeeing`))
      (:`1`
        (`self.UpdateHearing`)))))

(fn `UserConstructionScript`)