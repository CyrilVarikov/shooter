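; AI controller for the wolf that turns AI Perception updates into Blackboard state.
; Each perceived actor becomes the aim target if it is damageable, not tagged Wolf, and the wolf is neither attacking nor has the player in melee range.
; Stimuli are read by array index: the first sets player visibility, the second sets investigation state and target location.
; BeginPlay delays caching the pawn to work around perception bugs.
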(event `self.ReceiveBeginPlay`
  ;[1 1 1] This delay needed to fix bugs with AI perception
  (`KismetSystemLibrary.Delay` 0.2)
  (set `self.ControlledPawn` (`self.K2_GetPawn`)))

(event `self.AIPerception.OnPerceptionUpdated`
  (params (UpdatedActors :type "Array of Actor Object Reference (by ref)"))
  (for _array_element UpdatedActors
    (bind _info (`AIPerceptionComponent.GetActorsPerception` (`self.AIPerception`) _array_element))
    (`self.CompleteSenses` (break `ActorPerceptionBlueprintInfo` _info) (`.LastSensedStimuli` (break `ActorPerceptionBlueprintInfo` _info)))))

(fn `CompleteSenses`
  (params (AimActor :type "Actor Object Reference") (Stimulus :type "Array of AIStimulus Structure"))
  (locals (LocalSense :type "AIStimulus Structure"))
  (bind (_age _expirationage _strength _stimuluslocation _receiverlocation _tag _bsuccessfullysensed) (break `AIStimulus` (`local.LocalSense`)))
  (`self.ConditionalSet` AimActor)
  (for (_array_element _array_index) Stimulus
    (set `local.LocalSense` _array_element)
    (switch `int` _array_index
      (:`0`
        (`BlackboardComponent.SetValueAsBool` (`AIBlueprintHelperLibrary.GetBlackboard` null) "CanSeePlayer" (`.bSuccessfullySensed` (break `AIStimulus` (`local.LocalSense`)))))
      (:`1`
        (`BlackboardComponent.SetValueAsBool` (`AIBlueprintHelperLibrary.GetBlackboard` null) "IsInvestigating" _bsuccessfullysensed)
        (`BlackboardComponent.SetValueAsVector` (`AIBlueprintHelperLibrary.GetBlackboard` null) "TargetLocation" _stimuluslocation)))))

(fn `UserConstructionScript`)