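; AI controller for the zombie boss that starts its pawn roaming after spawn.
; On BeginPlay it waits briefly, prints a spawn message, caches the controlled AI_Zombie_Boss and sets PauseBeforeStart.
; Tick waits for that flag, which acts as a ready signal despite its name, then calls the pawn's Roam once through a DoOnce.
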(event `self.ReceiveBeginPlay`
  (`KismetSystemLibrary.Delay` 0.2)
  (`KismetSystemLibrary.PrintString` "Boss Spawned" true true (struct :`R` 0.020501 :`G` 0.066947 :`B` 1.0 :`A` 1.0))
  (bind _asai_zombie_boss (cast `/Game/AI/AI_Zombie_Boss` (`self.K2_GetPawn`)))
  (set `self.ControlledPawn` _asai_zombie_boss)
  (set `self.PauseBeforeStart` true))

(event `self.ReceiveTick`
  (params (DeltaSeconds :type "Float (single-precision)"))
  (if (`self.PauseBeforeStart`)
    (`/Engine/EditorBlueprintResources/StandardMacros.DoOnce` false
      (:`Completed`
        (`/Game/AI/AI_Zombie_Boss.Roam` (`self.ControlledPawn`))))))

(fn `UserConstructionScript`)