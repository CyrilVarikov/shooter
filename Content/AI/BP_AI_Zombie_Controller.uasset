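; AI controller for the zombie enemy, driving it with the BT_Zombie behavior tree started on BeginPlay.
; AI perception updates on the TopDownCharacter write the sensing result to the CanSeePlayer blackboard key.
; Tick holds a one-shot Roam call gated by PauseBeforeStart, but the delayed setup that sets that flag and caches the controlled zombie is disconnected and never runs.
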(event `self.ReceiveBeginPlay`
  (`self.RunBehaviorTree` "/Game/AI/BT_Zombie.BT_Zombie"))

(event `self.ReceiveTick`
  (params (DeltaSeconds :type "Float (single-precision)"))
  (if (`self.PauseBeforeStart`)
    (`/Engine/EditorBlueprintResources/StandardMacros.DoOnce` false
      (:`Completed`
        (`/Game/AI/AI_Zombie.Roam` (`self.ControlledZombie`))))))

(event `self.AIPerception.OnTargetPerceptionUpdated`
  (params (Actor :type "Actor Object Reference") (Stimulus :type "AIStimulus Structure"))
  (cast `/Game/TopDownBP/Blueprints/TopDownCharacter` Actor)
  (`BlackboardComponent.SetValueAsBool` (`AIBlueprintHelperLibrary.GetBlackboard` null) "CanSeePlayer" (`.bSuccessfullySensed` (break `AIStimulus` Stimulus))))

(fn `UserConstructionScript`)