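; BP_FBBox is a box actor that shifts along the world X axis through two custom events.
; LFMove targets 200 units toward negative X from the LRCube component's world location, and RBMove targets 200 toward positive X.
; Each event makes a single non-swept SetActorLocation through VInterpTo with large fixed delta and speed values, so the box jumps straight to the target instead of gliding.
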(event `/Game/World/IMoveInterface.LFMove`
  (bind _returnvalue (`SceneComponent.K2_GetComponentLocation` (`self.LRCube`)))
  (`self.K2_SetActorLocation` (`KismetMathLibrary.VInterpTo` _returnvalue (- _returnvalue (200.0 0.0 0.0)) 200.0 50.0)))

(event `/Game/World/IMoveInterface.RBMove`
  (bind _returnvalue (`SceneComponent.K2_GetComponentLocation` (`self.LRCube`)))
  (`self.K2_SetActorLocation` (`KismetMathLibrary.VInterpTo` _returnvalue (+ _returnvalue (200.0 0.0 0.0)) 15.0 200.0)))

(fn `UserConstructionScript`)