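; BP_Blade is a world hazard that damages TopDownCharacter actors touching it.
; Entering its Box casts the overlapping actor, stores it as LastOverlaped and passes a fixed negative amount to its CustomDamageEvent.
; Tick runs through a one-second Delay, repeating that damage while the stored character still overlaps the blade.
; Only the most recently stored character receives the repeated damage.
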(event `self.ReceiveActorBeginOverlap`
  (params (OtherActor :type "Actor Object Reference")))

(event `self.Box.OnComponentBeginOverlap`
  (params (OverlappedComponent :type "PrimitiveComponent Object Reference") (OtherActor :type "Actor Object Reference") (OtherComp :type "PrimitiveComponent Object Reference") (OtherBodyIndex :type Integer) (bFromSweep :type Boolean) (SweepResult :type "HitResult Structure (by ref)"))
  (bind _astop_down_character (cast `/Game/TopDownBP/Blueprints/TopDownCharacter` OtherActor))
  (set `self.LastOverlaped` _astop_down_character)
  (`/Game/TopDownBP/Blueprints/TopDownCharacter.CustomDamageEvent` _astop_down_character -25.0 null))

(event `self.ReceiveTick`
  (params (DeltaSeconds :type "Float (single-precision)"))
  (bind _lastoverlaped (`self.LastOverlaped`))
  (`KismetSystemLibrary.Delay` 1.0)
  (if (`self.IsOverlappingActor` _lastoverlaped)
    (bind _astop_down_character (cast `/Game/TopDownBP/Blueprints/TopDownCharacter` _lastoverlaped))
    (set `self.LastOverlaped` _astop_down_character)
    (`/Game/TopDownBP/Blueprints/TopDownCharacter.CustomDamageEvent` _astop_down_character -25.0 null)))

(fn `UserConstructionScript`)