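; BP_MovementTrap is a trap actor that slows zombies on overlap.
; On begin overlap, actors of exact class AI_Zombie have their walk speed reduced by a fixed amount through ChangeSpeed, with debug prints.
; End overlap instead checks for AI_Zombie_Boss before setting a fixed walk speed, so regular zombies stay slowed.
; A delayed self-destroy chain is unconnected and never runs.
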(event `self.ReceiveBeginPlay`)

(event `self.ReceiveActorBeginOverlap`
  (params (OtherActor :type "Actor Object Reference"))
  ;[1 1 1] Get in trap
  (`KismetSystemLibrary.PrintString` "123")
  (if (== (`GameplayStatics.GetObjectClass` OtherActor) "/Game/AI/AI_Zombie.AI_Zombie_C")
    (bind _asai_zombie (cast `/Game/AI/AI_Zombie` OtherActor))
    (`KismetSystemLibrary.PrintString` "Trapped")
    (`self.ChangeSpeed` _asai_zombie -300.0)))

(event `self.ReceiveActorEndOverlap`
  (params (OtherActor :type "Actor Object Reference"))
  ;[1 1 1] Get out the trap
  (if (== (`GameplayStatics.GetObjectClass` OtherActor) "/Game/AI/AI_Zombie_Boss.AI_Zombie_Boss_C")
    (bind _asai_zombie (cast `/Game/AI/AI_Zombie` OtherActor))
    (set `CharacterMovementComponent.MaxWalkSpeed` 500.0 (`Character.CharacterMovement` _asai_zombie))))

(fn `UserConstructionScript`)