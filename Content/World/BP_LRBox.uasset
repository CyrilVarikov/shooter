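; BP_LRBox is a moving hazard box that travels back and forth between start and finish target points.
; On Tick, MoveMacro eases it toward the selected point with VInterpTo, without sweep.
; A Delay after each Tick move flips the MoveStart flag about every two seconds, so reversal is time-based rather than on arrival.
; Any actor that begins overlapping it takes damage, and a debug string prints.
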(event `self.ReceiveActorBeginOverlap`
  (params (OtherActor :type "Actor Object Reference"))
  (`GameplayStatics.ApplyDamage` OtherActor (`self.Damage`))
  (`KismetSystemLibrary.PrintString` "Hello"))

(event `self.ReceiveTick`
  (params (DeltaSeconds :type "Float (single-precision)"))
  (`self.MoveMacro` DeltaSeconds
    (:`Completed`
      (`KismetSystemLibrary.Delay` 2.0)
      (set `self.MoveStart` (not (`self.MoveStart`))))))

(fn `UserConstructionScript`)