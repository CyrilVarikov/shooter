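; BP_Jumpad_bonus is a pickup that adds one to the player character's jumpad count.
; Its Sphere stops simulating physics on its first hit, so it stays where it lands.
; When a TopDownCharacter, matched by exact class, overlaps SphereCollision, the bonus increments that character's CountOfJumpad and destroys itself.
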(event `self.Sphere.OnComponentHit`
  (params (HitComponent :type "PrimitiveComponent Object Reference") (OtherActor :type "Actor Object Reference") (OtherComp :type "PrimitiveComponent Object Reference") (NormalImpulse :type "Vector Structure") (Hit :type "HitResult Structure (by ref)"))
  (`PrimitiveComponent.SetSimulatePhysics` (`self.Sphere`) false))

(event `self.Sphere collision.OnComponentBeginOverlap`
  (params (OverlappedComponent :type "PrimitiveComponent Object Reference") (OtherActor :type "Actor Object Reference") (OtherComp :type "PrimitiveComponent Object Reference") (OtherBodyIndex :type Integer) (bFromSweep :type Boolean) (SweepResult :type "HitResult Structure (by ref)"))
  (if (== (`GameplayStatics.GetObjectClass` OtherActor) "/Game/TopDownBP/Blueprints/TopDownCharacter.TopDownCharacter_C")
    (bind _astop_down_character (cast `/Game/TopDownBP/Blueprints/TopDownCharacter` OtherActor))
    (bind _result (`/Engine/EditorBlueprintResources/StandardMacros.IncrementInt` (`/Game/TopDownBP/Blueprints/TopDownCharacter.CountOfJumpad` _astop_down_character))
      (:`  `
        (set `/Game/TopDownBP/Blueprints/TopDownCharacter.CountOfJumpad` _result _astop_down_character)
        (`self.K2_DestroyActor`)))))

(fn `UserConstructionScript`)